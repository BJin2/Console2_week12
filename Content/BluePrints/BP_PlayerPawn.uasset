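; BP_PlayerPawn is the player pawn Blueprint that manages the local player's HUD widgets.
; On BeginPlay, if locally controlled, it creates player, damage and pickup widgets and binds weapon ammo changes to update the player UI's weapon icon and ammo counts.
; Tick shows the pickup UI in place of the player UI while a pickable weapon is valid, resetting the player UI's material properties when it returns.
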(event `OnAmmoChange` :!signature `self.OnWeaponAmmoChange`
  (params (weaponTexture :type "Texture2D Object Reference") (ammoCount :type "Float (double-precision)") (maxAmmo :type "Float (double-precision)"))
  (`/Game/BluePrints/PlayerUI.SetWeaponIcon` (stale `self.ReceiveBeginPlay` _returnvalue) weaponTexture ammoCount maxAmmo))

(event `self.ReceiveBeginPlay`
  (if (`self.IsLocallyControlled`)
    (bind _asplayer_controller (cast `PlayerController` (`self.GetController`)))
    (`self.SetOwner` _asplayer_controller self)
    (`|ExecutionSequence`
      (:`then_0`
        (bind _returnvalue (`|CreateWidget` "/Game/BluePrints/PlayerUI.PlayerUI_C" _asplayer_controller))
        (bind _output_get (set `self.PlayerUI` _returnvalue))
        (`UserWidget.AddToViewport` _output_get 0)
        (add `self.OnWeaponAmmoChange` (delegate `OnAmmoChange`)))
      (:`then_1`
        (bind _returnvalue_2 (`|CreateWidget` "/Game/BluePrints/DamageUI.DamageUI_C" _asplayer_controller))
        (bind _output_get_2 (set `self.DamageUI` _returnvalue_2))
        (`UserWidget.AddToViewport` _output_get_2 0))
      (:`then_2`
        (bind _returnvalue_3 (`|CreateWidget` "/Game/BluePrints/PickupUI.PickupUI_C" _asplayer_controller))
        (bind _output_get_3 (set `self.PickupUI` _returnvalue_3))
        (`UserWidget.AddToViewport` _output_get_3 0)))))

(event `self.ReceiveTick`
  (params (DeltaSeconds :type "Float (single-precision)"))
  (bind _playerui (`self.PlayerUI`))
  (bind _pickupui (`self.PickupUI`))
  (bind _playerui_2 (`self.PlayerUI`))
  (bind _pickupui_2 (`self.PickupUI`))
  (if (`self.IsLocallyControlled`)
    (`self.pickableWeapon`
      (:`then`
        (`|ExecutionSequence`
          (:`then_0`
            (if (`Widget.IsInViewport` _playerui_2)
              (`Widget.RemoveFromParent` _playerui_2)))
          (:`then_1`
            (if (not (`Widget.IsInViewport` _pickupui_2))
              (`UserWidget.AddToViewport` _pickupui_2 0)))))
      (:`else`
        (`|ExecutionSequence`
          (:`then_0`
            (if (`Widget.IsInViewport` _pickupui)
              (`Widget.RemoveFromParent` _pickupui)))
          (:`then_1`
            (if (not (`Widget.IsInViewport` _playerui))
              (`UserWidget.AddToViewport` _playerui 0)
              (bind _asplayer_ui (cast `/Game/BluePrints/PlayerUI` _playerui))
              (`/Game/BluePrints/PlayerUI.ResetMaterialProperties` _asplayer_ui))))))))

(fn `UserConstructionScript`)