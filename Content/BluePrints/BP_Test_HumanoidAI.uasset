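; Test humanoid AI Blueprint that runs the Test_BT_V2 behavior tree against the player.
; On BeginPlay, only with authority, it starts the tree, writes player pawn 0 to the TargetActor blackboard key and binds an empty death handler.
; Unconnected logic would free the blackboard's CoverSpot if this AI occupies it and disable movement avoidance, but it never runs.
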(event `self.ReceiveBeginPlay`
  (bind _returnvalue (`AIBlueprintHelperLibrary.GetAIController` self))
  (if (`|EnumEquality` (`self.GetLocalRole`) "ROLE_Authority")
    (`AIController.RunBehaviorTree` _returnvalue "/Game/AI/Test_BT_V2.Test_BT_V2")
    (`BlackboardComponent.SetValueAsObject` (`AIBlueprintHelperLibrary.GetBlackboard` _returnvalue) "TargetActor" (`GameplayStatics.GetPlayerPawn` 0))
    (add `self.OnDeath` (delegate `On_Death_Event`))))

(event `On_Death_Event` :!signature `self.OnDeath`
  (params (actor :type "TPSCharacter Object Reference")))

(fn `UserConstructionScript`)